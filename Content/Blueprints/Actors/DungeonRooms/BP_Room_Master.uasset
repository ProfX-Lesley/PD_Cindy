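; BP_Room_Master is a dungeon room Blueprint that organizes collision zones, end points and spawn points under component groups.
; Its construction script calls a temporary debug function, marked for deletion before shipping, that makes each group's direct children and the ForwardLocalX component visible in game.
; The event graph holds only disabled placeholder events, so the file contains no runtime logic.
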(fn `Debugging: DELETE BEFORE SHIPPING`
  (for _array_element (`SceneComponent.GetChildrenComponents` (`self.CollisionZones_Grp`) false)
    (`SceneComponent.SetHiddenInGame` (`self.Forward (local x+)`) false false)
    (`SceneComponent.SetHiddenInGame` _array_element false false))
  (for _array_element_2 (`SceneComponent.GetChildrenComponents` (`self.EndPoints_Grp`) false)
    (`SceneComponent.SetHiddenInGame` _array_element_2 false false))
  (for _array_element_3 (`SceneComponent.GetChildrenComponents` (`self.SpawnPoints_Grp`) false)
    (`SceneComponent.SetHiddenInGame` _array_element_3 false false)))

(fn `UserConstructionScript`
  (`self.Debugging: DELETE BEFORE SHIPPING`))