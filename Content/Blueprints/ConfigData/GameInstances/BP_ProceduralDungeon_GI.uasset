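; Game instance for procedural dungeon generation that sets up a seeded random stream and spawns the starting room.
; An interface-style InitializeDungeonIF event first processes LoadingSeed: zero randomizes SeedStream and stores the resulting seed, while any other value seeds the stream directly.
; It then draws a room class from StartRoomClasses through that stream, making the choice reproducible per seed, and spawns it at StartRoomSpawnPoint.
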(event `/Game/Blueprints/Interfaces/BPI_ProceduralDungeon.InitializeDungeon_IF`
  (`self.ProcessSeedInput`)
  (`self.GenerateStarterRoom`))

(fn `GenerateStarterRoom`
  (`|SpawnActorFromClass` (`self.RandomizeStartRoom`) (`self.StartRoomSpawnPoint`) "Undefined" "MultiplyWithRoot" null null) ; Spawns in the Starting Room
)

(fn `ProcessSeedInput`
  (bind _loadingseed (`self.LoadingSeed`))
  (bind _seedstream (`self.SeedStream`))
  (bind _seedstream_initialseed (`KismetMathLibrary.BreakRandomStream` (`self.SeedStream`)))
  (if (== _loadingseed 0)
    (`KismetMathLibrary.SeedRandomStream` _seedstream) ; Similar to a variable Setter, but with\nmore functionality.\nThis sets the random seed to be a\nrandom value.
    (set `self.LoadingSeed` _seedstream_initialseed) ; Used as a reference of the seed...
    (else
      (`KismetMathLibrary.SetRandomStreamSeed` _seedstream _loadingseed) ; Also similar to a variable setter\nwith more functionality.\nLooks at the User's inputted number,\nthen sets it as the random seed.
    )))

(fn `RandomizeStartRoom`
  (returns (StartRoomClass :type "/Game/Blueprints/Actors/DungeonRooms/BP_Room_Master Class Reference"))
  (bind _startroomclasses (`self.StartRoomClasses`))
  (return (`|GetArrayItem` _startroomclasses (`KismetMathLibrary.RandomIntegerInRangeFromStream` (`self.SeedStream`) 0 (- (`KismetArrayLibrary.Array_Length` _startroomclasses) 1)))))